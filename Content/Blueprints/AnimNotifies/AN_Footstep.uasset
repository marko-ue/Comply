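; Footstep anim notify that plays a step sound for Comply player and enemy characters during animation.
; It casts the mesh owner to the player or enemy class and skips the sound while that character's movement component is falling.
; The player uses a fixed footstep cue, while enemies use their own FootstepsSound.
; The sound always plays at the right-foot socket location.
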(fn `Received_Notify`
  (params (MeshComp :type "SkeletalMeshComponent Object Reference") (Animation :type "AnimSequenceBase Object Reference") (EventReference :type "AnimNotifyEventReference Structure (by ref)"))
  (returns (ReturnValue :type Boolean))
  (bind _ascomply_player_character (cast `ComplyPlayerCharacter` (`ActorComponent.GetOwner` MeshComp))
    (:`then`
      (if (not (`NavMovementInterface.IsFalling` (`Pawn.GetMovementComponent` _ascomply_player_character)))
        (`GameplayStatics.PlaySoundAtLocation` "/Game/Assets/Audio/Player/Footsteps/PlayerFootsteps_Cue.PlayerFootsteps_Cue" (`SceneComponent.GetSocketLocation` MeshComp "foot_r") (struct) 1.0 1.0 0.0 null null null null)
        (return false)))
    (:`CastFailed`
      (bind _ascomply_enemy_character (cast `ComplyEnemyCharacter` (`ActorComponent.GetOwner` MeshComp)))
      (if (not (`NavMovementInterface.IsFalling` (`Pawn.GetMovementComponent` _ascomply_enemy_character)))
        (`GameplayStatics.PlaySoundAtLocation` (`ComplyEnemyCharacter.FootstepsSound` _ascomply_enemy_character) (`SceneComponent.GetSocketLocation` MeshComp "foot_r") (struct) 1.0 1.0 0.0 null null null null)
        (return false)))))