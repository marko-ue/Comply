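; Player character Blueprint for the Ranger, holding a HUD overlay setup and debug hotkeys.
; On BeginPlay it creates a WBP_Overlay widget and adds it to the viewport.
; Debug key Z prints every gameplay tag owned by its Ability System Component, and debug key X calls DownPlayer to down the character.
; The construction script is empty and the overlap event is an unused stub.
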(event EventBeginPlay
  (bind _returnvalue (UserInterface|CreateWidget "/Game/Blueprints/UI/WBP_Overlay.WBP_Overlay_C"))
  (UserInterface|Viewport|AddtoViewport _returnvalue 0))

(event Collision|EventActorBeginOverlap
  (params (OtherActor :type Actor%20Object%20Reference)))

(event Input|KeyboardEvents|DebugKeyX
  (params (Key :type Key%20Structure :default "None") (ActionValue :type Input%20Action%20Value%20Structure))
  (:Pressed
    (Class|ComplyPlayerCharacter|DownPlayer)))

(event Input|KeyboardEvents|DebugKeyZ
  (params (Key :type Key%20Structure :default "None") (ActionValue :type Input%20Action%20Value%20Structure))
  (:Pressed
    (for _array_element (GameplayTags|BreakGameplayTagContainer (GameplayTags|GetOwnedGameplayTags (Ability|GetAbilitySystemComponent 0) :!class /Script/GameplayTags.BlueprintGameplayTagLibrary))
      (Development|PrintString (Utilities|String|ToString(Name) (GameplayTags|GetTagName _array_element)) true true "(R=0.838201,G=0.000000,B=1.000000,A=1.000000)" 5.0))))

(fn ConstructionScript)